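; BP_LotManager is a lot manager Blueprint that adds a name label and a debug readout on top of its parent class.
; The construction script floats a text render of the lot name above the grid center.
; Every tick it prints a one-frame on-screen summary of mesh section counts for the grid, terrain, wall, floor and water components, plus the RoomManager's room count.
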(event `self.ReceiveTick`
  (params (DeltaSeconds :type "Float (single-precision)"))
  (`parent.ReceiveTick` DeltaSeconds)
  (`KismetSystemLibrary.PrintText` (`|FormatText` "[Mesh] \nGridSections: {grids} \nTerrainSections {terrains} \nWallSections: {walls} \nFloorSections: {floors} \nWaterSections: {waters} \n------------------------- \n[Data] \nRooms: {rooms}" (`ProceduralMeshComponent.GetNumSections` (`self.GridComponent`)) (`ProceduralMeshComponent.GetNumSections` (`self.TerrainComponent`)) (`ProceduralMeshComponent.GetNumSections` (`self.WallComponent`)) (`ProceduralMeshComponent.GetNumSections` (`self.FloorComponent`)) (`RoomManagerComponent.GetRoomCount` (`self.RoomManager`)) (`ProceduralMeshComponent.GetNumSections` (`self.WaterComponent`))) true false (struct :`G` 0.66 :`B` 1.0 :`A` 1.0) 0.0))

(event `self.ReceiveBeginPlay`
  (`parent.ReceiveBeginPlay`))

(fn `UserConstructionScript`
  (bind (_returnvalue_x _returnvalue_y _returnvalue_z) (`KismetMathLibrary.BreakVector` (`self.GridCenter`)))
  (`parent.UserConstructionScript`)
  (`SceneComponent.K2_SetWorldLocation` (`self.TextRender`) (`KismetMathLibrary.MakeVector` _returnvalue_x _returnvalue_y (+ _returnvalue_z 700.0)) false false)
  (`TextRenderComponent.K2_SetText` (`self.TextRender`) (`self.LotName`)))