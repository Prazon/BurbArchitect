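; Player controller for lot building: creates the base HUD and routes input to the possessed BurbPawn and its current build tool.
; Mouse move, select, cancel, delete and rotate inputs go to the tool via validity-checking macros, with pointer actions ignored over UI.
; A server event blocking-loads the requested tool class, spawns it and assigns it to the pawn.
; Other keys handle quick save/load, grid toggling, isometric rotation and camera mode.
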(event `Key|Nine`
  (params (Key :type "Key Structure"))
  (:`Pressed`
    (`self.QuickSave`)))

(event `Key|Zero`
  (params (Key :type "Key Structure"))
  (:`Pressed`
    (`self.QuickLoad`)))

(event `self.ReceiveBeginPlay`
  ;[1 1 1] BeginPlay
  (if (`self.IsLocalController`)
    (bind _returnvalue (`|CreateWidget` "/BurbArchitect/Widgets/W_BaseHUD.W_BaseHUD_C" self))
    (bind _output_get (set `self.BaseHUD` _returnvalue))
    (`UserWidget.AddToViewport` _output_get 0)
    (`WidgetBlueprintLibrary.SetInputMode_GameAndUIEx` self (`self.BaseHUD`) "DoNotLock" false)))

(event `self.ReceivePossess`
  (params (PossessedPawn :type "Pawn Object Reference"))
  ;[1 1 1] Possessed
  (bind _asbp_burb_pawn (cast `/BurbArchitect/Core/BP_BurbPawn` PossessedPawn))
  (set `self.CurrentPawn` _asbp_burb_pawn))

(event `InputAxisKey|MouseY` :consume false
  (params (AxisValue :type "Float (single-precision)"))
  ;[1 1 1] MouseMove
  (`self.IsHoveredUI` :!label _label
    (:`Exit`
      (bind _current_build_tool (`self.GetBuildTool`)
        (:`Is Valid`
          (`BuildTool.ServerMove` _current_build_tool (`self.CursorWorldLocation`) (`self.bSelectPressed`) (`self.CursorWorldHitResult`) (`self.LastTracedLevel`)))))))

(event `InputAxisKey|MouseX` :consume false
  (params (AxisValue :type "Float (single-precision)"))
  ;[1 1 1] MouseMove
  (goto _label))

(event `InputAction|Select`
  (params (Key :type "Key Structure"))
  ;[1 1 1] Select
  (:`Pressed`
    (`self.IsHoveredUI`
      (:`Exit`
        (set `self.bSelectPressed` true)
        (bind _current_build_tool (`self.GetBuildTool`)
          (:`Is Valid`
            (`BuildTool.ServerClick` _current_build_tool))))))
  (:`Released`
    (`self.IsHoveredUI`
      (:`Exit`
        (set `self.bSelectPressed` false)
        (bind _current_build_tool_2 (`self.GetBuildTool`)
          (:`Is Valid`
            (`BuildTool.ServerRelease` _current_build_tool_2)))))))

(event `Key|Escape`
  (params (Key :type "Key Structure"))
  ;[1 1 1] Cancel
  (:`Pressed`
    (bind _current_build_tool (`self.GetBuildTool`)
      (:`Is Valid`
        (`BuildTool.ServerCancel` _current_build_tool)))))

(event `Key|Delete`
  (params (Key :type "Key Structure"))
  ;[1 1 1] Deletion Mode
  (:`Pressed`
    (bind _current_build_tool (`self.GetBuildTool`)
      (:`Is Valid`
        (`BuildTool.ServerDelete` _current_build_tool)))))

(event `InputAction|RotateToolRight`
  (params (Key :type "Key Structure"))
  ;[1 1 1] Tool rotations
  (:`Pressed`
    (bind _current_build_tool (`self.GetBuildTool`)
      (:`Is Valid`
        (`BuildTool.RotateRight` _current_build_tool)))))

(event `InputAction|ToggleGrid`
  (params (Key :type "Key Structure"))
  ;[1 1 1] Toggle GridLines
  (:`Pressed`
    (bind _isa (`/Engine/EditorBlueprintResources/StandardMacros.FlipFlop`)
      (:`A`
        _)
      (:`B`
        _))
    (`LotManager.ToggleGrid` (`self.GetCurrentLot`) (not _isa))))

(event `InputAction|RotateToolLeft`
  (params (Key :type "Key Structure"))
  ;[1 1 1] Tool rotations
  (:`Pressed`
    (bind _current_build_tool (`self.GetBuildTool`)
      (:`Is Valid`
        (`BuildTool.RotateLeft` _current_build_tool)))))

(event `InputAction|RotateRight`
  (params (Key :type "Key Structure"))
  (:`Pressed`
    (bind _asburb_pawn (`self.GetBurbPawn`))
    (`BurbPawn.RotateIsometricLeft` _asburb_pawn)))

(event `InputAction|RotateLeft`
  (params (Key :type "Key Structure"))
  (:`Pressed`
    (bind _asburb_pawn (`self.GetBurbPawn`))
    (`BurbPawn.RotateIsometricRight` _asburb_pawn)))

(event `Server: TryCreateBuildTool`
  (params (NewBuildTool :type "BuildTool Soft Class Reference"))
  (bind _returnvalue (`self.K2_GetPawn`))
  (bind _returnvalue_location (`KismetMathLibrary.BreakTransform` (`self.GetTransform` (`self.K2_GetPawn`))))
  (bind _asburb_pawn (cast `BurbPawn` _returnvalue :!pure true))
  (bind _returnvalue_2 (`KismetSystemLibrary.LoadClassAsset_Blocking` NewBuildTool))
  (bind _asbuild_tool (castclass `BuildTool` _returnvalue_2))
  (bind _returnvalue_3 (`|SpawnActorFromClass` _asbuild_tool (`KismetMathLibrary.MakeTransform` _returnvalue_location) "AlwaysSpawn" "MultiplyWithRoot" _asburb_pawn null _asburb_pawn _returnvalue))
  (bind _asburb_pawn_2 (cast `BurbPawn` (`self.K2_GetPawn`)))
  (`BurbPawn.SetCurrentBuildTool` _asburb_pawn_2 _returnvalue_3))

(event `Key|I`
  (params (Key :type "Key Structure"))
  (:`Pressed`
    (bind _asburb_pawn (`self.GetBurbPawn`))
    (`BurbPawn.ToggleCameraMode` _asburb_pawn)))

(fn `GetCurrentLot`
  (returns (`Current Lot` :type "LotManager Object Reference"))
  (bind _asburb_pawn (cast `BurbPawn` (`self.K2_GetPawn`)))
  (bind _currentlot (`BurbPawn.CurrentLot` _asburb_pawn)
    (:`then`
      (return _currentlot))
    (:`else`)))

(fn `UserConstructionScript`)