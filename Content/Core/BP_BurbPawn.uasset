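; BP_BurbPawn is the player's camera pawn for building on lots, with yaw-relative movement, zoom, rotation, floor cycling and wall cutaway modes.
; Input events mostly call inherited functions, pass Shift and floor placement toggles to the current build tool, and route undo/redo to the BuildServer.
; On possession it binds to the controller's level-change event and takes the player's name.
; Debug aids show the current tool, wall mode and a toggleable room-view widget.
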(event `self.ReceiveTick`
  (params (DeltaSeconds :type "Float (single-precision)"))
  (bind _currentbuildtool (`self.CurrentBuildTool`))
  (`parent.ReceiveTick` DeltaSeconds)
  (`KismetSystemLibrary.PrintText` (`|FormatText` "CurrentTool: {tool}" (select `bool` (`KismetSystemLibrary.IsValid` _currentbuildtool) :`false` "none" :`true` (`KismetSystemLibrary.GetDisplayName` _currentbuildtool))) true false (struct :`R` 1.0 :`B` 0.745933 :`A` 1.0) 0.0))

(event `self.ReceivePossessed`
  (params (NewController :type "Controller Object Reference"))
  ;[1 1 1] Possessed
  (bind _asbp_burb_player_controller (cast `/BurbArchitect/Core/BP_BurbPlayerController` NewController))
  (add `/BurbArchitect/Core/BP_BurbPlayerController.OnLevelChanged` _asbp_burb_player_controller (`|CreateDelegate` :!event `HandleOnLevelChanged`))
  (set `self.DisplayName` (`KismetTextLibrary.Conv_StringToText` (`PlayerState.GetPlayerName` (`Controller.PlayerState` _asbp_burb_player_controller)))))

(event `Key|LeftShift`
  (params (Key :type "Key Structure"))
  ;[1 1 1] Shift modifier
  (:`Pressed`
    (bind _currentbuildtool (`self.CurrentBuildTool`)
      (:`then`
        (set `BuildTool.bShiftPressed` true _currentbuildtool))
      (:`else`)))
  (:`Released`
    (bind _currentbuildtool_2 (`self.CurrentBuildTool`)
      (:`then`
        (set `BuildTool.bShiftPressed` false _currentbuildtool_2))
      (:`else`))))

(event `InputAxis|MoveRight`
  (params (AxisValue :type "Float (single-precision)"))
  (bind (_returnvalue_roll _returnvalue_pitch _returnvalue_yaw) (`KismetMathLibrary.BreakRotator` (`SceneComponent.K2_GetComponentRotation` (`self.Camera`))))
  ;[0.04688 0.04688 0.04688] Move Right/Left
  (`self.AddMovementInput` self (`KismetMathLibrary.GetRightVector` (`KismetMathLibrary.MakeRotator` 0.0 0.0 _returnvalue_yaw)) AxisValue true))

(event `InputAction|FloorModifier`
  (params (Key :type "Key Structure"))
  ;[1 1 1] Floor Modifier
  (:`Pressed`
    (bind _currentbuildtool (`self.CurrentBuildTool` :!label _label)
      (:`then`
        (bind _asbp_floor_tool (cast `/BurbArchitect/BuildTools/BP_FloorTool` _currentbuildtool))
        (set `BuildFloorTool.PlacementMode` (select `EFloorPlacementMode` (`BuildFloorTool.PlacementMode` _asbp_floor_tool) :`FullTile` "SingleTriangle" :`SingleTriangle` "FullTile" :!type "EFloorPlacementMode Enum") _asbp_floor_tool))
      (:`else`))))

(event `Key|P`
  (params (Key :type "Key Structure"))
  (:`Pressed`
    (bind _debug_room_widget (`self.debug_room_widget`)
      (:`then`
        (`Widget.RemoveFromParent` _debug_room_widget)
        (set `self.debug_room_widget` null))
      (:`else`
        (bind _returnvalue (`|CreateWidget` "/BurbArchitect/Widgets/W_Debug_RoomView.W_Debug_RoomView_C" null (`self.CurrentLot`) (`self.CurrentLevel`)))
        (bind _output_get (set `self.debug_room_widget` _returnvalue))
        (`UserWidget.AddToViewport` _output_get 999)))))

(event `InputAction|ZoomOut`
  (params (Key :type "Key Structure"))
  ;[1 1 1] CameraZoom
  (:`Pressed`
    (`self.ZoomOut`)))

(event `InputAction|ZoomIn`
  (params (Key :type "Key Structure"))
  ;[1 1 1] CameraZoom
  (:`Pressed`
    (`self.ZoomIn`)))

(event `Key|Alt+F`
  (params (Key :type "Key Structure"))
  ;[1 1 1] Floor Modifier
  (:`Pressed`
    (goto _label)))

(event `InputAxis|MoveForward`
  (params (AxisValue :type "Float (single-precision)"))
  (bind (_returnvalue_roll _returnvalue_pitch _returnvalue_yaw) (`KismetMathLibrary.BreakRotator` (`SceneComponent.K2_GetComponentRotation` (`self.Camera`))))
  ;[0.04688 0.04688 0.04688] Move Forward/Backwards
  (`self.AddMovementInput` self (`KismetMathLibrary.GetForwardVector` (`KismetMathLibrary.MakeRotator` 0.0 0.0 _returnvalue_yaw)) AxisValue true))

(event `Key|RightMouseButton` :consume false
  (params (Key :type "Key Structure"))
  ;[0 0 0] CameraRotation
  (:`Pressed`
    (set `self.bRotateButtonPressed` true))
  (:`Released`
    (set `self.bRotateButtonPressed` false)))

(event `InputAxis|RotHoz`
  (params (AxisValue :type "Float (single-precision)"))
  ;[0 0 0] CameraRotation
  (`self.RotateHorizontal` AxisValue))

(event `InputAxis|RotVert`
  (params (AxisValue :type "Float (single-precision)"))
  ;[0 0 0] CameraRotation
  (`self.RotateVertical` AxisValue))

(event `InputAction|WallsUp`
  (params (Key :type "Key Structure"))
  ;[1 1 1] Wall Cutaway modes
  (:`Pressed`
    (`self.PreviousCutawayMode`)
    (`self.ApplyCutawayMode` (`.Rotation` (`Controller.GetPlayerViewPoint` (`GameplayStatics.GetPlayerController` 0))) :!label _label_2)
    (`KismetSystemLibrary.PrintText` (`|FormatText` "WallMode: {mode}" (`|GetEnumeratorNameAsString` (`self.CutawayMode`))))))

(event `InputAction|Undo`
  (params (Key :type "Key Structure"))
  (bind _returnvalue (subsystem `BuildServer`))
  ;[1 1 1] UndoRedo
  (:`Pressed`
    (if (`BuildServer.CanUndo` _returnvalue)
      (`BuildServer.Undo` _returnvalue))))

(event `InputAction|WallsDown`
  (params (Key :type "Key Structure"))
  ;[1 1 1] Wall Cutaway modes
  (:`Pressed`
    (`self.NextCutawayMode`)
    (goto _label_2)))

(event `InputAction|CycleFloorUp`
  (params (Key :type "Key Structure"))
  ;[1 1 1] Change floors
  (:`Pressed`
    (`self.MoveUpFloor`)))

(event `InputAction|Redo`
  (params (Key :type "Key Structure"))
  (bind _returnvalue (subsystem `BuildServer`))
  ;[1 1 1] UndoRedo
  (:`Pressed`
    (if (`BuildServer.CanRedo` _returnvalue)
      (`BuildServer.Redo` _returnvalue))))

(event `InputAction|CycleFloorDown`
  (params (Key :type "Key Structure"))
  ;[1 1 1] Change floors
  (:`Pressed`
    (`self.MoveDownFloor`)))

(fn `FindUnownedLot`
  (bind _returnvalue (`GameplayStatics.GetActorOfClass` "/Script/BurbArchitect.LotManager"))
  (set `self.CurrentLot` _returnvalue))

(fn `UserConstructionScript`)