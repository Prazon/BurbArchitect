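; BP_FloorTool is a build tool for placing floor pieces, working through a preview floor mesh.
; Its Delete event destroys the preview floor and calls the parent delete, and EndPlay also removes that temporary preview.
; Left Shift sets a held flag, and the FloorModifier input toggles placement between full tile and single triangle.
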(event `self.Delete`
  (bind _previewfloormesh (`self.PreviewFloorMesh`)
    (:`then`
      (`FloorComponent.DestroyFloor` _previewfloormesh)
      (`parent.Delete`))
    (:`else`)))

(event `self.ReceiveEndPlay`
  (params (EndPlayReason :type "EEndPlayReason Enum" :default "Destroyed"))
  ;[1 1 1] EndPlay - Destroy temp floor
  (bind _previewfloormesh (`self.PreviewFloorMesh`)
    (:`then`
      (`FloorComponent.DestroyFloor` _previewfloormesh))
    (:`else`)))

(event `Key|LeftShift`
  (params (Key :type "Key Structure"))
  (:`Pressed`
    (set `self.bShiftPressed` true))
  (:`Released`
    (set `self.bShiftPressed` false)))

(event `InputAction|FloorModifier`
  (params (Key :type "Key Structure"))
  (:`Pressed`
    (set `self.PlacementMode` (select `EFloorPlacementMode` (`self.PlacementMode`) :`FullTile` "SingleTriangle" :`SingleTriangle` "FullTile" :!type "EFloorPlacementMode Enum"))))

(fn `UserConstructionScript`)