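; BP_PortalBase is a portal base actor that tracks whether its placement is clear of other portals.
; Each tick it queries its Box for overlapping BP_PortalBase actors, excludes itself, and sets Valid to true only when none remain.
; Its construction script enables hidden shadow casting on every static mesh component, so the meshes can still cast shadows while hidden.
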(event `self.ReceiveTick`
  (params (DeltaSeconds :type "Float (single-precision)"))
  (`parent.ReceiveTick` DeltaSeconds)
  (bind _output_get (set `self.Overlapping Actors` (`PrimitiveComponent.GetOverlappingActors` (`self.Box`) "BP_PortalBase_C")))
  (`KismetArrayLibrary.Array_RemoveItem` _output_get self)
  (if (> (`KismetArrayLibrary.Array_Length` _output_get) 0)
    (set `self.bValid` false)
    (else
      (set `self.bValid` true))))

(fn `UserConstructionScript`
  (for _array_element (`self.K2_GetComponentsByClass` "/Script/Engine.StaticMeshComponent")
    (if (not (`PrimitiveComponent.bCastHiddenShadow` _array_element))
      (`PrimitiveComponent.SetCastHiddenShadow` _array_element true))))